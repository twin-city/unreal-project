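; BP_LightLine is a Blueprint that procedurally lays out a straight row of static meshes, with variables named for trees despite the asset's name.
; The Construction Script loops over NumberOfTree, adding components spaced along local X by SpaceBetweenTrees.
; Each gets a small random height offset and random yaw, unseeded, so the variation rerolls on reconstruction.
; The event graph has no active logic.
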(event EventBeginPlay)

(event Collision|EventActorBeginOverlap
  (params (OtherActor :type Actor%20Object%20Reference)))

(event EventTick
  (params (DeltaSeconds :type Float%20%28single-precision%29)))

(fn ConstructionScript
  (for _index (range 0 (Variables|Default|GetNumberOfTree))
    (AddComponent|AddStaticMeshComponent false (Math|Transform|MakeTransform (Math|Vector|MakeVector (Math|Conversions|ToFloat(Integer) (* _index (Variables|Default|GetSpaceBetweenTrees))) 0.0 (Math|Conversions|ToFloat(Integer) (Math|Random|RandomInteger 10))) (Math|Rotator|MakeRotator 0.0 0.0 (.yaw (Math|Random|RandomRotator false))) "1.000000,1.000000,1.000000"))))